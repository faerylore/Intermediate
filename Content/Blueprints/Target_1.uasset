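; Target actor that changes the colour of the level's RandomLight actors when shot with the first-person projectile.
; On BeginPlay it caches all RandomLight actors in an array.
; A projectile hit on the Target component loops through that array and calls ChangeLightColour on each light.
; Disconnected leftover nodes hold unused bullseye distance checks, self-destruction and direct point light colour randomisation.
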(event OnComponentHit(Target)
  (params (HitComponent :type Primitive%20Component%20Object%20Reference) (OtherActor :type Actor%20Object%20Reference) (OtherComp :type Primitive%20Component%20Object%20Reference) (NormalImpulse :type Vector :default "0, 0, 0") (Hit :type Hit%20Result%20Structure%20%28by%20ref%29))
  (Utilities|Casting|CastToBP_FirstPersonProjectile OtherActor)
  (for _array_element (stale EventBeginPlay _output_get)
    (Default|ChangeLightColour _array_element)))

(event EventBeginPlay
  (bind _outactors (Actor|GetAllActorsOfClass "/Game/Blueprints/RandomLight.RandomLight_C"))
  (bind _output_get (Variables|Default|SetRandomLights _outactors)))

(event Collision|EventActorBeginOverlap
  (params (OtherActor :type Actor%20Object%20Reference)))

(event EventTick
  (params (DeltaSeconds :type Float%20%28single-precision%29)))

(fn ConstructionScript)