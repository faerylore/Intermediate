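; Moving shooting target that drops Gems and destroys itself when hit by a BP_FirstPersonProjectile.
; The SideToSide timeline, started on BeginPlay, offsets it along world X from its start position, calling Reverse on every update.
; Hit distance to the Point component is printed and sets the reward: two randomly offset Gems for a near-center hit, otherwise one.
; Alternate Y-axis movement and geometry collection nodes are left unconnected.
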(event OnComponentHit(Target)
  (params (HitComponent :type Primitive%20Component%20Object%20Reference) (OtherActor :type Actor%20Object%20Reference) (OtherComp :type Primitive%20Component%20Object%20Reference) (NormalImpulse :type Vector :default "0, 0, 0") (Hit :type Hit%20Result%20Structure%20%28by%20ref%29))
  (bind _returnvalue (Transformation|GetActorLocation))
  (bind _returnvalue_2 (Transformation|GetActorLocation))
  (bind _returnvalue_3 (Transformation|GetActorLocation))
  (bind _point (Variables|Default|GetPoint))
  (bind _returnvalue_4 (Transformation|GetWorldLocation _point))
  (bind _returnvalue_5 (Math|Vector|Distance(Vector) (.location Hit) _returnvalue_4))
  (Utilities|Casting|CastToBP_FirstPersonProjectile OtherActor)
  (Development|PrintString (Utilities|String|ToString(Float) _returnvalue_5))
  (if (< _returnvalue_5 2e+01)
    (Game|SpawnActorfromClass "/Game/Blueprints/Gems.Gems_C" (Math|Conversions|ToTransform(Vector) (Math|Vector|MakeVector (Math|Random|RandomFloatinRange (.x _returnvalue) (+ (.x _returnvalue) 3e+01)) (Math|Random|RandomFloatinRange (.y _returnvalue) (+ (.y _returnvalue) 3e+01)) (Math|Random|RandomFloatinRange (.z _returnvalue) (+ (.z _returnvalue) 3e+01)))) "Undefined" "MultiplyWithRoot" 0 0)
    (Game|SpawnActorfromClass "/Game/Blueprints/Gems.Gems_C" (Math|Conversions|ToTransform(Vector) (Math|Vector|MakeVector (Math|Random|RandomFloatinRange (.x _returnvalue_2) (+ (.x _returnvalue_2) 3e+01)) (Math|Random|RandomFloatinRange (.y _returnvalue_2) (+ (.y _returnvalue_2) 3e+01)) (Math|Random|RandomFloatinRange (.z _returnvalue_2) (+ (.z _returnvalue_2) 3e+01)))) "Undefined" "MultiplyWithRoot" 0 0)
    (Actor|DestroyActor)
    (else
      (Game|SpawnActorfromClass "/Game/Blueprints/Gems.Gems_C" (Math|Conversions|ToTransform(Vector) (Math|Vector|MakeVector (Math|Random|RandomFloatinRange (.x _returnvalue_3) (+ (.x _returnvalue_3) 3e+01)) (Math|Random|RandomFloatinRange (.y _returnvalue_3) (+ (.y _returnvalue_3) 3e+01)) (Math|Random|RandomFloatinRange (.z _returnvalue_3) (+ (.z _returnvalue_3) 3e+01)))) "Undefined" "MultiplyWithRoot" 0 0)
      (Actor|DestroyActor))))

(event EventBeginPlay
  (bind _returnvalue (Transformation|GetActorLocation))
  (Variables|Default|SetStartLocation (.x _returnvalue))
  (bind _offset (Timeline|SideToSide PlayFromStart)
    (:Update
      (Transformation|SetActorLocation (Math|Vector|MakeVector (+ (Variables|Default|GetStartLocation) (* 1e+02 _offset)) (.y _returnvalue) (.z _returnvalue)) false false)
      (Timeline|SideToSide Reverse))))

(fn ConstructionScript)