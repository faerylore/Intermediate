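; Gem pickup actor that the first-person character collects by overlapping its collider, raising that character's GemCount.
; When the count reaches exactly seven in FirstPersonMap, it spawns a Portal at a hardcoded transform.
; It then destroys itself and prints a debug message, as it does for other counts.
; At seven in any other map, the gem is neither destroyed nor followed by a portal.
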(event OnComponentBeginOverlap(Collider)
  (params (OverlappedComponent :type Primitive%20Component%20Object%20Reference) (OtherActor :type Actor%20Object%20Reference) (OtherComp :type Primitive%20Component%20Object%20Reference) (OtherBodyIndex :type Integer) (bFromSweep :type Boolean) (SweepResult :type Hit%20Result%20Structure%20%28by%20ref%29))
  (bind _asbp_first_person_character (Utilities|Casting|CastToBP_FirstPersonCharacter OtherActor))
  (bind _output_get (Variables|/Game/FirstPerson/Blueprints/BP_FirstPersonCharacter.BP_FirstPersonCharacter_C|SetGem_Count _asbp_first_person_character (+ (Variables|/Game/FirstPerson/Blueprints/BP_FirstPersonCharacter.BP_FirstPersonCharacter_C|GetGem_Count _asbp_first_person_character) 1)))
  (if (== _output_get 7)
    (bind _returnvalue (Game|GetCurrentLevelName true))
    (if (Utilities|Enum|Equal(Enum) _returnvalue "FirstPersonMap")
      (Game|SpawnActorfromClass "/Game/Blueprints/Portal.Portal_C" (Math|Transform|MakeTransform "310.000000,370.000000,170.000000" "0.000000,-50.000000,0.000000" "1.000000,1.000000,1.000000") "Undefined" "MultiplyWithRoot" 0 0)
      (Actor|DestroyActor :!label _label)
      (Development|PrintString "cURRENCY ADDED"))
    (else
      (goto _label))))

(fn ConstructionScript)