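; Moving shootable target that rewards accurate hits from the first-person projectile with gems.
; A looping Timeline lerps the Target component from the actor's start location toward TargetLocation, transformed by the current actor transform.
; Projectile hits near Point spawn two randomly offset Gems, while other projectile hits run a spawn with no class shown; both destroy the actor.
; Hit distance is debug-printed, and geometry collection logic is left unconnected.
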(event OnComponentHit(Target)
  (params (HitComponent :type Primitive%20Component%20Object%20Reference) (OtherActor :type Actor%20Object%20Reference) (OtherComp :type Primitive%20Component%20Object%20Reference) (NormalImpulse :type Vector :default "0, 0, 0") (Hit :type Hit%20Result%20Structure%20%28by%20ref%29))
  (bind _returnvalue (Transformation|GetActorLocation))
  (bind _returnvalue_2 (Transformation|GetActorLocation))
  (bind _point (Variables|Default|GetPoint))
  (bind _returnvalue_3 (Transformation|GetWorldLocation _point))
  (bind _returnvalue_4 (Math|Vector|Distance(Vector) (.location Hit) _returnvalue_3))
  (Utilities|Casting|CastToBP_FirstPersonProjectile OtherActor)
  (Development|PrintString (Utilities|String|ToString(Float) _returnvalue_4))
  (if (< _returnvalue_4 2e+01)
    (Game|SpawnActorfromClass "/Game/Blueprints/Gems.Gems_C" (Math|Conversions|ToTransform(Vector) (Math|Vector|MakeVector (Math|Random|RandomFloatinRange (.x _returnvalue) (+ (.x _returnvalue) 3e+01)) (Math|Random|RandomFloatinRange (.y _returnvalue) (+ (.y _returnvalue) 3e+01)) (Math|Random|RandomFloatinRange (.z _returnvalue) (+ (.z _returnvalue) 3e+01)))) "Undefined" "MultiplyWithRoot" 0 0)
    (Game|SpawnActorfromClass "/Game/Blueprints/Gems.Gems_C" (Math|Conversions|ToTransform(Vector) (Math|Vector|MakeVector (Math|Random|RandomFloatinRange (.x _returnvalue_2) (+ (.x _returnvalue_2) 3e+01)) (Math|Random|RandomFloatinRange (.y _returnvalue_2) (+ (.y _returnvalue_2) 3e+01)) (Math|Random|RandomFloatinRange (.z _returnvalue_2) (+ (.z _returnvalue_2) 3e+01)))) "Undefined" "MultiplyWithRoot" 0 0)
    (Actor|DestroyActor)
    (else
      (Game|SpawnActorfromClass "/Game/Blueprints/Gems.Gems_C" (Math|Transform|MakeTransform (Transformation|GetWorldLocation (Variables|Default|GetTarget)) "0, 0, 0" "1.000000,1.000000,1.000000") "Undefined" "MultiplyWithRoot" 0 0)
      (Actor|DestroyActor))))

(event EventBeginPlay
  (Variables|Default|SetStarting%20Location (Transformation|GetActorLocation))
  (bind _newtrack_0 (Timeline|Timeline Play)
    (:Update
      (Transformation|SetWorldLocation (Variables|Default|GetTarget) (Math|Vector|Lerp(Vector) (Variables|Default|GetStarting%20Location) (Math|Transform|TransformLocation (Transformation|GetActorTransform) (Variables|Default|GetTarget%20Location)) _newtrack_0) false false))
    (:Finished
      (Utilities|FlowControl|DelayUntilNextTick)
      (Timeline|Timeline PlayFromStart))))

(fn ConstructionScript)